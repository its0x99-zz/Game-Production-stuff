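; Player character for a 2D side-scrolling platformer, with running, dashing, jumping, trace-based wall jumps, ladder climbing and projectile attacks.
; Tick picks the flipbook through a priority-based state function and flips the sprite by X velocity.
; Timelines drive squash-and-stretch with dust on jump and landing, plus mushroom growth.
; Damage reduces health until the actor is destroyed; ring-drop and shrink-on-hit logic is unconnected, and dash animation keys off IsFalling.
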(event `self.ReceiveBeginPlay`
  ;[1 1 1] Begin Play
  (bind _asgame_controller_bp (cast `/Game/Blueprints/Misc/GameControllerBP` (`GameplayStatics.GetGameMode`)))
  (set `self.GameController` _asgame_controller_bp))

(event `UpdateAnimation`
  (bind _returnvalue (`NavMovementComponent.IsFalling` (`self.CharacterMovement`)))
  ;[1 1 1] Control Animation
  (set `self.bIsMoving` (> (`KismetMathLibrary.VSize` (`self.GetVelocity`)) 0.0))
  (bind _outputfb (`self.AnimationStateMachine` (`self.bIsMoving`) _returnvalue _returnvalue (`self.bIsAttacking`) (`self.bIsClimbing`)))
  (`PaperFlipbookComponent.SetFlipbook` (`self.Sprite`) _outputfb))

(event `self.ReceiveTick`
  (params (DeltaSeconds :type "Float (single-precision)"))
  ;[1 1 1] Update
  (`self.UpdateAnimation`)
  (`/Engine/EditorBlueprintResources/StandardMacros.CompareFloat` (.x (`MovementComponent.Velocity` (`self.CharacterMovement`)))
    (:`>`
      (`SceneComponent.K2_SetRelativeRotation` :`self` (`self.Sprite`)))
    (:`<`
      (`SceneComponent.K2_SetRelativeRotation` (`self.Sprite`) (struct :`Yaw` 180.0) false false))))

(event `InputAxis|MoveRight`
  (params (AxisValue :type "Float (single-precision)"))
  ;[1 1 1] Movement Control
  (if (`self.bCanMoveRight`)
    (`self.AddMovementInput` (1.0 0.0 0.0) AxisValue)))

(event `InputAction|Dash`
  (params (Key :type "Key Structure"))
  (bind _returnvalue (`self.GetVelocity`))
  ;[1 1 1] Dash
  (:`Pressed`
    (if (!= _returnvalue (0.0 0.0 0.0))
      (if (`NavMovementComponent.IsFalling` (`self.CharacterMovement`))
        (`self.LaunchCharacter` (* (+ _returnvalue (0.0 0.0 0.0)) (1.5 1.5 1.5)) true true)
        (else
          (`self.LaunchCharacter` (* (+ _returnvalue (0.0 0.0 1.0)) (1.5 1.5 250.0)) true true))))))

(event `InputAction|Jump`
  (params (Key :type "Key Structure"))
  ;[1 1 1] Jumping
  (:`Pressed`
    (set `self.bCanMoveRight` true)
    (if (`NavMovementComponent.IsFalling` (`self.CharacterMovement`))
      (`self.WallJump`)
      (else
        (`self.Jump`)
        (`self.JumpFX`))))
  (:`Released`
    (`self.StopJumping`)))

(event `self.OnLanded`
  (params (Hit :type "HitResult Structure (by ref)"))
  ;[1 1 1] Landed
  (`self.LandFx`))

(event `WallJump`
  (bind _returnvalue (`self.GetActorForwardVector`))
  (bind _returnvalue_x (`KismetMathLibrary.BreakVector` (`self.K2_GetActorLocation`)))
  ;[1 1 1] WallJump
  (bind (_outhit _returnvalue_2) (`KismetSystemLibrary.LineTraceSingle` (- (`self.K2_GetActorLocation`) (* _returnvalue (+ (`CapsuleComponent.GetScaledCapsuleRadius` (`self.CapsuleComponent`)) 15.0))) (+ (`self.K2_GetActorLocation`) (* _returnvalue (+ (`CapsuleComponent.GetScaledCapsuleRadius` (`self.CapsuleComponent`)) 15.0))) "TraceTypeQuery1" true))
  (if _returnvalue_2
    (`self.LaunchCharacter` (`KismetMathLibrary.MakeVector` (* (`KismetMathLibrary.SignOfFloat` (- _returnvalue_x (.x (`.Location` (`GameplayStatics.BreakHitResult` _outhit))))) 450.0) 0.0 (`CharacterMovementComponent.JumpZVelocity` (`self.CharacterMovement`))) true true)
    (`self.JumpFX`)
    (elif (< (`self.JumpCurrentCount`) (`self.JumpMaxCount`))
      (`self.Jump`)
      (`self.JumpFX`))))

(event `JumpFX`
  ;[1 1 1] Jump Effects
  (`GameplayStatics.SpawnEmitterAtLocation` "/Game/Art/Particles/pDust.pDust" (`SceneComponent.K2_GetComponentLocation` (`self.DustBox`)))
  (bind (_direction _squash) (`Timeline|Timeline_0` :!via `PlayFromStart`)
    (:`Update`
      (`self.SetActorScale3D` (`KismetMathLibrary.VLerp` (`self.CurrentScale`) (0.25 1.0 2.0) _squash)))))

(event `LandFx`
  ;[1 1 1] Jump Effects
  (`GameplayStatics.SpawnEmitterAtLocation` "/Game/Art/Particles/pDust.pDust" (`SceneComponent.K2_GetComponentLocation` (`self.DustBox`)))
  (bind (_direction _squash) (`Timeline|Timeline_1` :!via `PlayFromStart`)
    (:`Update`
      (`self.SetActorScale3D` (`KismetMathLibrary.VLerp` (`self.CurrentScale`) (2.0 1.0 0.25) _squash)))))

(event `InputAction|Fire`
  (params (Key :type "Key Structure"))
  ;[1 1 1] Attacking
  (:`Pressed`
    (if (not (`self.bIsAttacking`))
      (`self.AttackAnimation`))))

(event `FireProjectile`
  ;[1 1 1] Attacking
  (`|SpawnActorFromClass` "/Game/Blueprints/Misc/ProjectileBP.ProjectileBP_C" (`SceneComponent.K2_GetComponentToWorld` (`self.ProjectileSpawn`)) "AlwaysSpawn" "OverrideRootScale" null null))

(event `AttackAnimation`
  (bind _attackfb (`self.AttackFB`))
  ;[1 1 1] Attacking
  (`|ExecutionSequence`
    (:`then_0`
      (set `self.bIsAttacking` true)
      (`KismetSystemLibrary.Delay` 0.3)
      (`self.FireProjectile`))
    (:`then_1`
      (`KismetSystemLibrary.Delay` (/ (`KismetMathLibrary.Conv_IntToDouble` (`PaperFlipbook.GetNumFrames` _attackfb)) (`PaperFlipbook.FramesPerSecond` _attackfb)))
      (set `self.bIsAttacking` false))))

(event `InputAxis|MoveUp`
  (params (AxisValue :type "Float (single-precision)"))
  ;[1 1 1] Lader Logic
  (if (`self.bCanClimb`)
    (if (`KismetMathLibrary.InRange_FloatFloat` AxisValue -0.1 0.1)
      (`PaperFlipbookComponent.SetPlayRate` (`self.Sprite`) 0.0)
      (else
        (set `self.bIsClimbing` true)
        (set `self.bCanMoveRight` false)
        (`PaperFlipbookComponent.SetPlayRate` (`self.Sprite`) 1.0)
        (`CharacterMovementComponent.SetMovementMode` (`self.CharacterMovement`) "MOVE_Flying" 0)
        (`self.AddMovementInput` (0.0 0.0 0.5) AxisValue)))))

(event `ClimbingEnd`
  ;[1 1 1] Lader Logic
  (if (`self.bIsClimbing`)
    (`CharacterMovementComponent.SetMovementMode` (`self.CharacterMovement`) "MOVE_Walking" 0)
    (set `self.bIsClimbing` false)
    (set `self.bCanMoveRight` true)
    (`PaperFlipbookComponent.SetPlayRate` (`self.Sprite`) 1.0)))

(event `DropRing`
  (for _ (range (`/Game/Blueprints/Misc/GameControllerBP.RingsCollected` (`self.GameController`)))
    (`|SpawnActorFromClass` "/Game/Blueprints/PickUps/bpPickUpRing.bpPickUpRing_C" (`self.GetTransform`) "Undefined" "OverrideRootScale" null true null))
  (set `/Game/Blueprints/Misc/GameControllerBP.RingsCollected` 0 (`self.GameController`)))

(event `ScaleControl`
  (params (bIsHealth :type Boolean))
  ;[1 1 1] Health Size Swap
  (if bIsHealth
    (if (not (`/Game/Blueprints/Misc/GameControllerBP.bHasMushroom` (`self.GameController`)))
      (bind (_direction _scalelerp) (`Timeline|Scale`)
        (:`Update`
          (`self.SetActorScale3D` _scalelerp)
          (set `self.CurrentScale` (`self.IncreasedScale`))
          (set `/Game/Blueprints/Misc/GameControllerBP.bHasMushroom` true (`self.GameController`)))))
    (else
      (set `self.CurrentScale` (`self.StartScale`))
      (`self.SetActorScale3D` (`self.StartScale`))
      (set `/Game/Blueprints/Misc/GameControllerBP.bHasMushroom` false (`self.GameController`)))))

(event `self.ReceiveAnyDamage`
  (params (Damage :type "Float (single-precision)") (DamageType :type "DamageType Object Reference") (InstigatedBy :type "Controller Object Reference") (DamageCauser :type "Actor Object Reference"))
  ;[1 1 1] Death Function
  (set `self.Health` (- (`self.Health`) Damage))
  (if (not (> (`self.Health`) 0.0))
    (`GameplayStatics.SpawnEmitterAtLocation` "/Game/Art/Particles/pDust.pDust")
    (`self.K2_DestroyActor`)))

(fn `AnimationStateMachine`
  (params (bIsMoving :type Boolean) (bIsFalling :type Boolean) (bIsDashing :type Boolean) (bIsAttacking :type Boolean) (bIsClimbing :type Boolean))
  (returns (outputFB :type "PaperFlipbook Object Reference"))
  (locals (AnimationState :type "/Game/Data/AnimationState Enum"))
  (if bIsClimbing
    (set `local.AnimationState` "NewEnumerator6")
    (elif bIsDashing
      (set `local.AnimationState` "NewEnumerator3")
      (elif bIsAttacking
        (set `local.AnimationState` "NewEnumerator4")
        (elif bIsFalling
          (set `local.AnimationState` "NewEnumerator2")
          (elif bIsMoving
            (set `local.AnimationState` "NewEnumerator1")
            (else
              (set `local.AnimationState` "NewEnumerator0")))))))
  (return (select `/Game/Data/AnimationState` (`local.AnimationState`) :`NewEnumerator0` (`self.IdleFB`) :`NewEnumerator1` (`self.RunnginFB`) :`NewEnumerator2` (`self.JumpingFB`) :`NewEnumerator3` (`self.JumpingFB`) :`NewEnumerator4` (`self.AttackFB`) :`NewEnumerator6` (`self.ClimbingFB`))))

(fn `UserConstructionScript`
  (set `CharacterMovementComponent.JumpZVelocity` 400.0 (`self.CharacterMovement`))
  (set `self.JumpMaxHoldTime` 0.3)
  (bind _output_get (set `self.StartScale` (`self.GetActorScale3D`)))
  (set `self.CurrentScale` _output_get)
  (set `self.Health` (`self.MaxHealth`)))